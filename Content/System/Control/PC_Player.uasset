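; Player controller for Project Spark that drives a Generic_CHARA pawn and lets the player cycle through teammates.
; Input events handle yaw-relative movement, camera look and block/unblock; jump calls an empty stub, as are Move and PlayerStateMachine.
; Swapping destroys the current pawn, spawns the next class from the game instance's Teammates list at its location and rotation, then possesses it and restores control rotation.
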(event EventBeginPlay
  (bind _asgeneric_chara (Utilities|Casting|CastToGeneric_CHARA (Pawn|GetControlledPawn)))
  (Variables|Default|SetcontrolledPawn _asgeneric_chara))

(event EventTick
  (params (DeltaSeconds :type Float%20%28single-precision%29))
  (bind _asgi_project_spark (Utilities|Casting|CastToGI_ProjectSpark (Game|GetGameInstance)))
  (Variables|Default|SetGAME_INSTANCE _asgi_project_spark))

(event Input|ActionEvents|InputActionJump
  (params (Key :type Key%20Structure))
  (:Pressed
    (CallFunction|HandleJump)))

(event Input|ActionEvents|InputActionAction1
  (params (Key :type Key%20Structure))
  (bind _controlledpawn (Variables|Default|GetcontrolledPawn))
  (:Pressed
    (Default|Block _controlledpawn))
  (:Released
    (Default|Unblock _controlledpawn)))

(event Input|ActionEvents|InputActionSwapCharacters
  (params (Key :type Key%20Structure))
  (:Pressed
    (CallFunction|SwapCharacters)))

(event Input|AxisEvents|InputAxisForward
  (params (AxisValue :type Float%20%28single-precision%29))
  (bind _asgeneric_chara (Utilities|Casting|CastToGeneric_CHARA (Pawn|GetControlledPawn)))
  (Pawn|Input|AddMovementInput _asgeneric_chara (Math|Vector|GetForwardVector (Math|Rotator|MakeRotator 0.0 0.0 (.Yaw (Math|Rotator|BreakRotator (Pawn|GetControlRotation (Variables|Default|GetcontrolledPawn) :!class /Script/Engine.Pawn))))) AxisValue false))

(event Input|AxisEvents|InputAxisSide
  (params (AxisValue :type Float%20%28single-precision%29))
  (bind _asgeneric_chara (Utilities|Casting|CastToGeneric_CHARA (Pawn|GetControlledPawn)))
  (Pawn|Input|AddMovementInput _asgeneric_chara (Math|Vector|GetRightVector (Math|Rotator|MakeRotator 0.0 0.0 (.Yaw (Math|Rotator|BreakRotator (Pawn|GetControlRotation (Variables|Default|GetcontrolledPawn) :!class /Script/Engine.Pawn))))) AxisValue false))

(event Input|AxisEvents|InputAxisLookUp
  (params (AxisValue :type Float%20%28single-precision%29))
  (Class|PlayerController|AddPitchInput AxisValue))

(event Input|AxisEvents|InputAxisTurn
  (params (AxisValue :type Float%20%28single-precision%29))
  (Class|PlayerController|AddYawInput AxisValue))

(fn ConstructionScript)

(fn Move
  (params (input :type Float%20%28single-precision%29) (direction :type Vector)))

(fn HandleJump)

(fn PlayerStateMachine)

(fn SwapCharacters
  (LocalVariables|SetprevActorLoc (Transformation|GetActorLocation (Variables|Default|GetcontrolledPawn)))
  (LocalVariables|SetprevActorRot (Transformation|GetActorRotation (Variables|Default|GetcontrolledPawn)))
  (LocalVariables|SetprevControlRot (Pawn|GetControlRotation :!class /Script/Engine.Controller))
  (Actor|DestroyActor (Variables|Default|GetcontrolledPawn))
  (bind _nextchara (CallFunction|GetNextCharacter))
  (bind _returnvalue (Game|SpawnActorfromClass _nextchara (Math|Transform|MakeTransform (LocalVariables|GetprevActorLoc) (LocalVariables|GetprevActorRot)) "Undefined" 0 0))
  (Pawn|Possess _returnvalue)
  (Pawn|SetControlRotation (LocalVariables|GetprevControlRot))
  (Variables|Default|SetcontrolledPawn _returnvalue))

(fn GetNextCharacter
  (bind _game_instance (Variables|Default|GetGAME_INSTANCE))
  (bind _teammates (Variables|/Game/System/Flow/GI_ProjectSpark.GI_ProjectSpark_C|Getteammates _game_instance))
  (if (== (Variables|Default|GetcharacterIndex) (- (Utilities|Array|Length _teammates) 1))
    (Variables|Default|SetcharacterIndex 0)
    (else
      (Math|Integer|IncrementInt (Variables|Default|GetcharacterIndex)
        (:%20%20
          _))))
  (return (Utilities|Array|Get(acopy) _teammates (Variables|Default|GetcharacterIndex))))